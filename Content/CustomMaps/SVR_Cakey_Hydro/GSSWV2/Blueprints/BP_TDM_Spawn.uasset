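; BP_TDM_Spawn is a team deathmatch spawn actor that exists only in matching game modes.
; On BeginPlay the server checks whether the game mode's display name starts with TeamDeathMatch or TankTDM and destroys the actor otherwise.
; The construction script applies the TeamColor material to the TDMSpawn component to show its team.
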(event `self.ReceiveBeginPlay`
  (`/Engine/EditorBlueprintResources/ActorMacros.Switch Has Authority`
    (:`Authority`
      (if (not (or (`KismetStringLibrary.StartsWith` (`KismetSystemLibrary.GetDisplayName` (`GameplayStatics.GetGameMode`)) "TeamDeathMatch" "CaseSensitive") (`KismetStringLibrary.StartsWith` (`KismetSystemLibrary.GetDisplayName` (`GameplayStatics.GetGameMode`)) "TankTDM" "CaseSensitive")))
        (`self.K2_DestroyActor`)))))

(fn `UserConstructionScript`
  (`PrimitiveComponent.SetMaterial` (`self.TDM_Spawn`) 0 (`self.TeamColor`)))